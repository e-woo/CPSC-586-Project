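; Base enemy Blueprint that takes hits, suffers stacking bleed and drops rewards on death.
; Hits deal flat damage and add capped bleed stacks, stored in a map of ages that a looping timer advances, expires and converts to damage.
; Tick updates a camera-facing health and bleed widget.
; Death spawns XP, awards souls and sometimes drops a potion; a timed Scale function only prints a message.
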(event `self.ReceiveTick`
  (params (DeltaSeconds :type "Float (single-precision)"))
  (bind _statuswidget (`self.StatusWidget`))
  (bind _aswb_enemy_status (cast `/Game/Enemy/WB_EnemyStatus` (`WidgetComponent.GetWidget` (`self.StatusWidget`))))
  ;[1 1 1] Update enemy health bar
  (`ProgressBar.SetPercent` (`/Game/Enemy/WB_EnemyStatus.HeathBar` _aswb_enemy_status) (/ (`self.CurrentHealth`) (`self.MaxHealth`)))
  (if (> (`self.CurrentBleedStacks`) 0)
    (bind _bleedstack (`/Game/Enemy/WB_EnemyStatus.BleedStack` _aswb_enemy_status))
    (`Widget.SetVisibility` _bleedstack "Visible")
    (bind _bleedcount (`/Game/Enemy/WB_EnemyStatus.BleedCount` _aswb_enemy_status))
    (`Widget.SetVisibility` _bleedcount "Visible")
    (`TextBlock.SetText` _bleedcount (`KismetTextLibrary.Conv_StringToText` (`KismetStringLibrary.BuildString_Int` "" "x" (`self.CurrentBleedStacks`))))
    (else
      (`Widget.SetVisibility` _bleedstack "Hidden")
      (`Widget.SetVisibility` _bleedcount "Hidden")))
  (`SceneComponent.K2_SetWorldRotation` _statuswidget (`KismetMathLibrary.FindLookAtRotation` (`SceneComponent.K2_GetComponentLocation` _statuswidget) (`SceneComponent.K2_GetComponentLocation` (`PlayerCameraManager.TransformComponent` (`GameplayStatics.GetPlayerCameraManager` 0)))) false false))

(event `ApplyDamageToEnemy`
  (params (DamageTaken :type "Float (double-precision)") (MaxBleedStacks :type Integer))
  (set `self.DamageReceived` DamageTaken)
  (set `self.MaxBleedStacks` MaxBleedStacks)
  (`self.ApplyFlatDamage`)
  (`self.AddBleedStack`))

(event `ApplyFlatDamage`
  (set `self.CurrentHealth` (- (`self.CurrentHealth`) (`self.DamageReceived`)))
  (`self.CheckDeath`))

(event `AddBleedStack`
  ;[1 1 1] Add new bleed stack to enemy
  (if (not (== (`BlueprintMapLibrary.Map_Length` (`self.BleedStacks`)) (`self.MaxBleedStacks`)))
    (bind _result (`/Engine/EditorBlueprintResources/StandardMacros.IncrementInt` (`self.keyCount`))
      (:`  `
        (`BlueprintMapLibrary.Map_Add` (`self.BleedStacks`) _result)))))

(event `self.ReceiveBeginPlay`
  (bind _returnvalue (`KismetSystemLibrary.K2_SetTimerDelegate` (delegate `Bleed`) 1.0 true))
  (set `self.Timer` _returnvalue)
  (`KismetSystemLibrary.K2_SetTimer` self "Scale" 10.0 true))

(event `Bleed`
  (if (>= (`KismetSystemLibrary.K2_GetTimerElapsedTimeHandle` (`self.Timer`)) 1.0)
    (bind _keys (`BlueprintMapLibrary.Map_Keys` (`self.BleedStacks`)))
    (for _array_element _keys
      ;[1 1 1] Update all current bleed stacks on enemy
      (bind _result (`/Engine/EditorBlueprintResources/StandardMacros.IncrementInt` (`BlueprintMapLibrary.Map_Find` (`self.BleedStacks`) _array_element))
        (:`  `
          (if (>= _result (`self.BleedTimer`))
            (`BlueprintMapLibrary.Map_Remove` (`self.BleedStacks`) _array_element)
            (else
              (`BlueprintMapLibrary.Map_Add` (`self.BleedStacks`) _array_element _result))))))
    ;[1 1 1] Apply bleed damage
    (set `self.CurrentHealth` (- (`self.CurrentHealth`) (* (`BlueprintMapLibrary.Map_Length` (`self.BleedStacks`)) (* (`self.DamageReceived`) (`self.BleedDamageMultiplier`)))))
    (set `self.CurrentBleedStacks` (`BlueprintMapLibrary.Map_Length` (`self.BleedStacks`)))
    (`self.CheckDeath`)))

(fn `CheckDeath`
  (bind (_origin _boxextent) (`KismetSystemLibrary.GetComponentBounds` (`self.XPSpawnArea`)))
  (if (<= (`self.CurrentHealth`) 0.0)
    (for _ (range (+ (`self.XPDropAmount`) 1))
      ;[1 1 1] DropXP
      (`|SpawnActorFromClass` "/Game/Interaction/BP_ExperiencePoint.BP_ExperiencePoint_C" (`KismetMathLibrary.MakeTransform` (`KismetMathLibrary.RandomPointInBoundingBox` _origin _boxextent)) "AlwaysSpawn" "OverrideRootScale" null null))
    ;[1 1 1] Give souls to player
    (bind _asthird_person_character (cast `/Game/ThirdPersonBP/Blueprints/ThirdPersonCharacter` (`GameplayStatics.GetPlayerCharacter` 0)))
    (`/Game/ThirdPersonBP/Blueprints/ThirdPersonCharacter.ReceiveSouls` _asthird_person_character (`self.SoulReward`))
    ;[1 1 1] Spawn potion on death by chance
    (if (<= (`KismetMathLibrary.RandomFloat`) 0.1)
      (`|SpawnActorFromClass` "/Game/Interaction/Potions/BP_HealthPotion.BP_HealthPotion_C" (`KismetMathLibrary.MakeTransform` (`SceneComponent.K2_GetComponentLocation` (`self.CapsuleComponent`))) "Undefined" "OverrideRootScale" null null))
    (`self.K2_DestroyActor`)))

(fn `Scale`
  (`KismetSystemLibrary.PrintString` "base enemy scale"))

(fn `UserConstructionScript`)