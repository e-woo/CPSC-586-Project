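; Base pickup item actor that hands its HeldItem to the player character on Interact, then destroys itself.
; Overlapping its box as the player shows an Interact_UI prompt created at BeginPlay and fills in the world-space description text, and leaving clears both.
; Tick rotates the whole actor, not just the text, along the camera-to-description direction so the text tracks the player's view.
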(event `self.ReceiveBeginPlay`
  (bind _returnvalue (`|CreateWidget` "/Game/UI/Interact_UI.Interact_UI_C"))
  (set `self.Interact Prompt` _returnvalue))

(event `/Game/Interaction/BPI_Interaction.Interact`
  (params (PlayerCharacter :type "/Game/ThirdPersonBP/Blueprints/ThirdPersonCharacter Object Reference"))
  ;[1 1 1] Destroy item on pickup
  (`/Game/ThirdPersonBP/Blueprints/ThirdPersonCharacter.PickupItem` PlayerCharacter (`self.HeldItem`))
  (`self.K2_DestroyActor`))

(event `self.ReceiveTick`
  (params (DeltaSeconds :type "Float (single-precision)"))
  ;[1 1 1] Text look at player
  (`self.K2_SetActorRotation` (`KismetMathLibrary.MakeRotFromX` (- (`SceneComponent.K2_GetComponentLocation` (`self.Description`)) (`self.K2_GetActorLocation` (`GameplayStatics.GetPlayerCameraManager` 0))))))

(event `self.Box.OnComponentBeginOverlap`
  (params (OverlappedComponent :type "PrimitiveComponent Object Reference") (OtherActor :type "Actor Object Reference") (OtherComp :type "PrimitiveComponent Object Reference") (OtherBodyIndex :type Integer) (bFromSweep :type Boolean) (SweepResult :type "HitResult Structure (by ref)"))
  ;[1 1 1] Display text on overlap
  (if (== OtherActor (`GameplayStatics.GetPlayerCharacter` 0))
    (`UserWidget.AddToViewport` (`self.Interact Prompt`) 0)
    (`TextRenderComponent.K2_SetText` (`self.Description`) (`self.ItemDescription`))))

(event `self.Box.OnComponentEndOverlap`
  (params (OverlappedComponent :type "PrimitiveComponent Object Reference") (OtherActor :type "Actor Object Reference") (OtherComp :type "PrimitiveComponent Object Reference") (OtherBodyIndex :type Integer))
  ;[1 1 1] Display text on overlap
  (if (== (`GameplayStatics.GetPlayerCharacter` 0) OtherActor)
    (`Widget.RemoveFromParent` (`self.Interact Prompt`))
    (`TextRenderComponent.K2_SetText` (`self.Description`) (`KismetTextLibrary.GetEmptyText`))))

(fn `UserConstructionScript`)