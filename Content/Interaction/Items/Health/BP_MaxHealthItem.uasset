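; BP_MaxHealthItem is an item that permanently raises the player's maximum health when applied.
; Its ApplyItem event multiplies MaxHp by 1.1 and truncates the result to a whole number, leaving current HP unchanged.
; It then calls the player's EHealthUpdated dispatcher with current and new maximum health.
; BeginPlay and the construction script only defer to the parent class.
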(event `self.ReceiveBeginPlay`
  (`parent.ReceiveBeginPlay`))

(event `self.ApplyItem`
  (params (Player :type "/Game/ThirdPersonBP/Blueprints/ThirdPersonCharacter Object Reference"))
  (bind _output_get (set `/Game/ThirdPersonBP/Blueprints/ThirdPersonCharacter.MaxHp` (`KismetMathLibrary.Conv_IntToDouble` (`KismetMathLibrary.FTrunc` (* (`/Game/ThirdPersonBP/Blueprints/ThirdPersonCharacter.MaxHp` Player) 1.1))) Player))
  (`/Game/ThirdPersonBP/Blueprints/ThirdPersonCharacter.E_HealthUpdated` Player (`CharacterBase.CurrentHP` Player) _output_get))

(fn `UserConstructionScript`
  (`parent.UserConstructionScript`))