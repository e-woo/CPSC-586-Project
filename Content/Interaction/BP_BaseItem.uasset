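; Base pickup item that shows an interact prompt and detail widget while the player character overlaps its box.
; On BeginPlay it creates the prompt and copies its name and description into the ItemDetails widget via a cast to BPI_ItemDetails.
; Interact passes the item type to the player's PickupItem and destroys the actor, while ApplyItem is an empty event.
; Tick rotates the whole actor along the camera-to-icon direction as a billboard effect.
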(event `self.ReceiveBeginPlay`
  (bind _returnvalue (`|CreateWidget` "/Game/UI/Interact_UI.Interact_UI_C"))
  (set `self.Interact Prompt` _returnvalue)
  ;[1 1 1] Set the details of the item
  (bind _asbpi_item_details (cast `/Game/Interaction/BPI_ItemDetails` (`WidgetComponent.GetUserWidgetObject` (`self.ItemDetails`))))
  (set `/Game/Interaction/BPI_ItemDetails.Name` (`self.ItemName`) _asbpi_item_details)
  (set `/Game/Interaction/BPI_ItemDetails.Desc` (`self.ItemDescription`) _asbpi_item_details))

(event `ApplyItem`
  (params (Player :type "/Game/ThirdPersonBP/Blueprints/ThirdPersonCharacter Object Reference")))

(event `/Game/Interaction/BPI_InteractionPrompt.Interact`
  (params (PlayerCharacter :type "/Game/ThirdPersonBP/Blueprints/ThirdPersonCharacter Object Reference"))
  ;[1 1 1] Destroy item on pickup
  (`/Game/ThirdPersonBP/Blueprints/ThirdPersonCharacter.PickupItem` PlayerCharacter (`self.ItemType`))
  (`self.K2_DestroyActor`))

(event `self.ReceiveTick`
  (params (DeltaSeconds :type "Float (single-precision)"))
  ;[1 1 1] Have item always look at player
  (`self.K2_SetActorRotation` (`KismetMathLibrary.MakeRotFromX` (- (`SceneComponent.K2_GetComponentLocation` (`self.Icon`)) (`self.K2_GetActorLocation` (`GameplayStatics.GetPlayerCameraManager` 0))))))

(event `self.Box.OnComponentBeginOverlap`
  (params (OverlappedComponent :type "PrimitiveComponent Object Reference") (OtherActor :type "Actor Object Reference") (OtherComp :type "PrimitiveComponent Object Reference") (OtherBodyIndex :type Integer) (bFromSweep :type Boolean) (SweepResult :type "HitResult Structure (by ref)"))
  ;[1 1 1] Display text on overlap
  (if (== OtherActor (`GameplayStatics.GetPlayerCharacter` 0))
    (`UserWidget.AddToViewport` (`self.Interact Prompt`) 0)
    (`SceneComponent.SetHiddenInGame` (`self.ItemDetails`) false false)))

(event `self.Box.OnComponentEndOverlap`
  (params (OverlappedComponent :type "PrimitiveComponent Object Reference") (OtherActor :type "Actor Object Reference") (OtherComp :type "PrimitiveComponent Object Reference") (OtherBodyIndex :type Integer))
  ;[1 1 1] Display text on overlap
  (if (== (`GameplayStatics.GetPlayerCharacter` 0) OtherActor)
    (`Widget.RemoveFromParent` (`self.Interact Prompt`))
    (`SceneComponent.SetHiddenInGame` (`self.ItemDetails`) true false)))

(fn `UserConstructionScript`)