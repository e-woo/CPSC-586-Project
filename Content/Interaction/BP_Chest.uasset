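; Interactable chest that opens once and spawns a random item from its Items list.
; A box overlap shows an Interact_UI prompt to the first player's character while the chest is closed, and removes it on exit or interaction.
; Interact triggers OpenChest, where a timeline rotates the lid's roll, then spawns the item above the chest base when the animation finishes.
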(event `self.ReceiveBeginPlay`
  (bind _returnvalue (`|CreateWidget` "/Game/UI/Interact_UI.Interact_UI_C"))
  (set `self.Interact Prompt` _returnvalue))

(event `/Game/Interaction/BPI_InteractionPrompt.Interact`
  (params (PlayerCharacter :type "/Game/ThirdPersonBP/Blueprints/ThirdPersonCharacter Object Reference"))
  ;[1 1 1] Open chest on interact
  (if (not (`self.IsOpened?`))
    (`self.OpenChest`)
    (`Widget.RemoveFromParent` (`self.Interact Prompt`))))

(event `self.Box.OnComponentBeginOverlap`
  (params (OverlappedComponent :type "PrimitiveComponent Object Reference") (OtherActor :type "Actor Object Reference") (OtherComp :type "PrimitiveComponent Object Reference") (OtherBodyIndex :type Integer) (bFromSweep :type Boolean) (SweepResult :type "HitResult Structure (by ref)"))
  ;[1 1 1] Display text on overlap
  (if (`self.IsOpened?`)
    _
    (elif (== OtherActor (`GameplayStatics.GetPlayerCharacter` 0))
      (`UserWidget.AddToViewport` (`self.Interact Prompt`) 0))))

(event `self.Box.OnComponentEndOverlap`
  (params (OverlappedComponent :type "PrimitiveComponent Object Reference") (OtherActor :type "Actor Object Reference") (OtherComp :type "PrimitiveComponent Object Reference") (OtherBodyIndex :type Integer))
  ;[1 1 1] Display text on overlap
  (if (== (`GameplayStatics.GetPlayerCharacter` 0) OtherActor)
    (`Widget.RemoveFromParent` (`self.Interact Prompt`))))

(event `OpenChest`
  (bind _chesttop (`self.ChestTop`))
  (bind (_relativerotation_roll _relativerotation_pitch _relativerotation_yaw) (`KismetMathLibrary.BreakRotator` (`SceneComponent.RelativeRotation` _chesttop)))
  (set `self.IsOpened?` true)
  ;[1 1 1] Play chest opening animation
  (bind (_direction _lerp_value) (`Timeline|Timeline_OpenChest`)
    (:`Update`
      (`SceneComponent.K2_SetRelativeRotation` _chesttop (`KismetMathLibrary.MakeRotator` (`KismetMathLibrary.Lerp` 0.0 -110.0 _lerp_value) _relativerotation_pitch _relativerotation_yaw) false false))
    (:`Finished`
      ;[1 1 1] Spawn random item in chest
      (`|SpawnActorFromClass` (`KismetArrayLibrary.Array_Random` (`self.Items`)) (`KismetMathLibrary.MakeTransform` (+ (`SceneComponent.K2_GetComponentLocation` (`self.ChestBottom`)) (0.0 0.0 100.0))) "AlwaysSpawn" "OverrideRootScale" null null))))

(fn `UserConstructionScript`)