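; BP_HealthPotion is a single-use potion that restores health to the player when ApplyPotion is called on it.
; It heals by passing RestoreAmount into the player's DamagePlayer function, relying on negative damage, with a Used flag blocking repeat activation.
; A Niagara healing aura attaches to the player's mesh for a short delay, then the effect and the potion actor are destroyed.
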(event `self.ApplyPotion`
  (params (Player :type "/Game/ThirdPersonBP/Blueprints/ThirdPersonCharacter Object Reference"))
  ;[1 1 1] Restore health to player (Just apply -damage)
  (if (not (`self.Used?`))
    (set `self.Used?` true)
    (`/Game/ThirdPersonBP/Blueprints/ThirdPersonCharacter.DamagePlayer` Player (`self.RestoreAmount`))
    (bind _returnvalue (`NiagaraFunctionLibrary.SpawnSystemAttached` "/Game/MixedVFX/Particles/Mix/NS_HealingAura.NS_HealingAura" (`Character.Mesh` Player) "None" (0.0 0.0 0.0) (struct) "KeepRelativeOffset" true))
    (`KismetSystemLibrary.Delay` 2.0)
    (`ActorComponent.K2_DestroyComponent` _returnvalue)
    (`self.K2_DestroyActor`)))

(fn `UserConstructionScript`
  (`parent.UserConstructionScript`))